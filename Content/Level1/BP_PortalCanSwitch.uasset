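; BP_PortalCanSwitch is a level-exit portal that activates once every linked switch is on.
; InformTrigger checks the Switches array, then after a delay turns the screen emissive green and enables the trigger box's overlap events.
; The player pawn entering the trigger box loads the named level only while FrontColli is overlapped, gating entry by a second collision volume.
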(event `/Game/Level1/BI_InformTrigger.InformTrigger`
  (for _array_element (`self.Switches`)
    (if (`/Game/Level1/BP_BoardSwitch.IsSwitchOn` _array_element)
      (set `self.CanOpen` true)
      (else
        (set `self.CanOpen` false)
        (break))))
  (if (`self.CanOpen`)
    (`self.PortalOn`)))

(event `PortalOn`
  (`KismetSystemLibrary.Delay` (`self.Delay`))
  (`PrimitiveComponent.SetMaterial` (`self.Screen_Plane`) 0 "/Game/Level1/M_GreenEmiss.M_GreenEmiss")
  (set `PrimitiveComponent.bGenerateOverlapEvents` true (`self.TriggerBox`)))

(event `self.FrontColli.OnComponentBeginOverlap`
  (params (OverlappedComponent :type "PrimitiveComponent Object Reference") (OtherActor :type "Actor Object Reference") (OtherComp :type "PrimitiveComponent Object Reference") (OtherBodyIndex :type Integer) (bFromSweep :type Boolean) (SweepResult :type "HitResult Structure (by ref)"))
  (set `self.FrontColliTriggered` true))

(event `self.FrontColli.OnComponentEndOverlap`
  (params (OverlappedComponent :type "PrimitiveComponent Object Reference") (OtherActor :type "Actor Object Reference") (OtherComp :type "PrimitiveComponent Object Reference") (OtherBodyIndex :type Integer))
  (set `self.FrontColliTriggered` false))

(event `self.TriggerBox.OnComponentBeginOverlap`
  (params (OverlappedComponent :type "PrimitiveComponent Object Reference") (OtherActor :type "Actor Object Reference") (OtherComp :type "PrimitiveComponent Object Reference") (OtherBodyIndex :type Integer) (bFromSweep :type Boolean) (SweepResult :type "HitResult Structure (by ref)"))
  (if (== OtherActor (`GameplayStatics.GetPlayerPawn` 0))
    (if (`self.FrontColliTriggered`)
      (`GameplayStatics.OpenLevel` (`self.Level Name`)))))

(fn `UserConstructionScript`
  (`parent.UserConstructionScript`))