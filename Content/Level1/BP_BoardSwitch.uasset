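; BP_BoardSwitch is a pressure plate switch for Level1 whose board sinks when something overlaps its box collider and rises when the overlap ends.
; A timeline, played forward or reversed, lerps the board's relative Z offset.
; As the board crosses a depth threshold near the bottom, it toggles IsSwitchOn and calls InformSwitch only on state changes; InformSwitch is empty here.
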(event `BoardDown`
  (bind (_direction _updownanim) (`Timeline|UpDownAnim` :!label _label)
    (:`Update`
      (bind _returnvalue (`KismetMathLibrary.Lerp` 0.0 -19.0 _updownanim))
      (if (< _returnvalue -15.0)
        (if (not (`self.IsSwitchOn`))
          (bind _output_get (set `self.IsSwitchOn` true))
          (`self.InformSwitch` _output_get))
        (elif (`self.IsSwitchOn`)
          (bind _output_get_2 (set `self.IsSwitchOn` false))
          (`self.InformSwitch` _output_get_2)))
      (`SceneComponent.K2_SetRelativeLocation` (`self.Board`) (`KismetMathLibrary.MakeVector` 0.0 0.0 _returnvalue) false false))))

(event `BoardUp`
  (goto _label :!via `Reverse`))

(event `self.BoxColli.OnComponentBeginOverlap`
  (params (OverlappedComponent :type "PrimitiveComponent Object Reference") (OtherActor :type "Actor Object Reference") (OtherComp :type "PrimitiveComponent Object Reference") (OtherBodyIndex :type Integer) (bFromSweep :type Boolean) (SweepResult :type "HitResult Structure (by ref)"))
  (`self.BoardDown`))

(event `self.BoxColli.OnComponentEndOverlap`
  (params (OverlappedComponent :type "PrimitiveComponent Object Reference") (OtherActor :type "Actor Object Reference") (OtherComp :type "PrimitiveComponent Object Reference") (OtherBodyIndex :type Integer))
  (`self.BoardUp`))

(fn `InformSwitch`
  (params (IsSwitchOn :type Boolean)))

(fn `UserConstructionScript`)