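; BP_PickUpPutDown is an interactable actor that the player toggles between picked-up and put-down states, showing a Tips_PickUp prompt widget.
; Character overlap enables input on the actor and shows the prompt, while leaving overlap reverses both unless it is picked.
; The PickUp/PutDown action flips IsPicked and calls PickUp, also hiding the prompt, or PutDown.
; Both functions are empty here, leaving the actual carry behavior undefined.
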(event `self.ReceiveBeginPlay`
  (bind _returnvalue (`|CreateWidget` "/Game/Level1/Tips_PickUp.Tips_PickUp_C"))
  (bind _output_get (set `self.Tips_Pick` _returnvalue))
  (`UserWidget.AddToViewport` _output_get 0)
  (`Widget.SetVisibility` _output_get "Collapsed"))

(event `self.ReceiveActorBeginOverlap`
  (params (OtherActor :type "Actor Object Reference"))
  (cast `Character` OtherActor)
  (`self.EnableInput` (`GameplayStatics.GetPlayerController` 0))
  (`Widget.SetVisibility` (`self.Tips_Pick`) "Visible"))

(event `self.ReceiveActorEndOverlap`
  (params (OtherActor :type "Actor Object Reference"))
  (cast `Character` OtherActor)
  (if (not (`self.IsPicked`))
    (`self.DisableInput` (`GameplayStatics.GetPlayerController` 0))
    (`Widget.SetVisibility` (`self.Tips_Pick`) "Collapsed")))

(event `InputAction|PickUp/PutDown`
  (params (Key :type "Key Structure"))
  (:`Pressed`
    (if (`self.IsPicked`)
      (set `self.IsPicked` false)
      (`self.PutDown`)
      (else
        (set `self.IsPicked` true)
        (`Widget.SetVisibility` (`self.Tips_Pick`) "Collapsed")
        (`self.PickUp`)))))

(fn `PickUp`)

(fn `PutDown`)

(fn `UserConstructionScript`)