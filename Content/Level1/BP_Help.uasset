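; BP_Help is a Level 1 actor that shows a widget on screen while another actor overlaps it.
; On BeginPlay it creates the widget, adds it to the viewport and keeps it collapsed.
; Overlap begin makes the widget visible and hides the actor in game, and overlap end reverses both.
; The overlap events do not filter which actor triggers them.
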(event `self.ReceiveBeginPlay`
  (bind _returnvalue (`|CreateWidget` (`self.Class`)))
  (bind _output_get (set `self.MyWidget` _returnvalue))
  (`UserWidget.AddToViewport` _output_get 0)
  (`Widget.SetVisibility` _output_get "Collapsed"))

(event `self.ReceiveActorBeginOverlap`
  (params (OtherActor :type "Actor Object Reference"))
  (`Widget.SetVisibility` (`self.MyWidget`) "Visible")
  (`self.SetActorHiddenInGame` true))

(event `self.ReceiveActorEndOverlap`
  (params (OtherActor :type "Actor Object Reference"))
  (`Widget.SetVisibility` (`self.MyWidget`) "Collapsed")
  (`self.SetActorHiddenInGame` false))

(fn `UserConstructionScript`)