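; BP_JumpStage is a Level1 jump pad that unlocks once enough switches are on.
; InformTrigger counts the active entries in its Switches array and calls OpenJump when at least two are on.
; OpenJump turns the mesh green and enables overlap events on the sphere collider, which then moves any overlapping actor to a hard-coded destination.
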(event `/Game/Level1/BI_InformTrigger.InformTrigger`
  (set `self.SwitchOnNum` 0)
  (for _array_element (`self.Switches`)
    (if (`/Game/Level1/BP_BoardSwitch.IsSwitchOn` _array_element)
      (`/Engine/EditorBlueprintResources/StandardMacros.IncrementInt` (`self.SwitchOnNum`))))
  (if (>= (`self.SwitchOnNum`) 2)
    (`self.OpenJump`)))

(event `self.SphereColli.OnComponentBeginOverlap`
  (params (OverlappedComponent :type "PrimitiveComponent Object Reference") (OtherActor :type "Actor Object Reference") (OtherComp :type "PrimitiveComponent Object Reference") (OtherBodyIndex :type Integer) (bFromSweep :type Boolean) (SweepResult :type "HitResult Structure (by ref)"))
  (`self.K2_SetActorLocation` OtherActor (4154.0 -4725.0 3831.0) false false))

(fn `OpenJump`
  (`PrimitiveComponent.SetMaterial` (`self.StaticMeshComponent`) 0 "/Game/Level1/M_Green.M_Green")
  (set `PrimitiveComponent.bGenerateOverlapEvents` true (`self.SphereColli`)))

(fn `UserConstructionScript`)