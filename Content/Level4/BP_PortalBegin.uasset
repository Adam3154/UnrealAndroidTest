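; Level 4 entry portal that opens once every linked switch is on and sends actors to the portal manager's end portal.
; InformTrigger checks the switches, then runs a camera cutaway that enables the manager's tick, swaps the portal material and arms the trigger, and switches the player to first-person.
; Overlapping actors facing within 90 degrees of its forward are teleported via BP_PortalManager; the portal then disarms and resets all BI_Reset actors.
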(event `self.ReceiveBeginPlay`
  (bind _outactors (`GameplayStatics.GetAllActorsOfClass` "/Game/Level4/BP_PortalManager.BP_PortalManager_C"))
  (set `self.MyManager` (`|GetArrayItem` _outactors))
  (set `PrimitiveComponent.bGenerateOverlapEvents` false (`self.TriggerBox`)))

(event `/Game/Level1/BI_InformTrigger.InformTrigger`
  (for _array_element (`self.Switches`)
    (if (`/Game/Level1/BP_BoardSwitch.IsSwitchOn` _array_element)
      (set `self.CanPortal` true)
      (else
        (set `self.CanPortal` false)
        (break))))
  (if (`self.CanPortal`)
    (`self.PortalON`)
    (bind _asbpc_reverse_time (cast `/Game/Level1/BPC_ReverseTime` (`GameplayStatics.GetPlayerPawn` 0)))
    (`/Game/Level1/BPC_ReverseTime.ChangeToFPP` _asbpc_reverse_time)))

(event `PortalON`
  (`PlayerController.SetViewTargetWithBlend` (`GameplayStatics.GetPlayerController` 0) (`self.Camera`) 1.0 "VTBlend_Linear" 0.0 false)
  (`KismetSystemLibrary.Delay` 1.5)
  (`self.SetActorTickEnabled` (`self.MyManager`) true)
  (`PrimitiveComponent.SetMaterial` (`self.Portal`) 0 "/Game/Level4/M_PortalEnd.M_PortalEnd")
  (set `PrimitiveComponent.bGenerateOverlapEvents` true (`self.TriggerBox`))
  (`KismetSystemLibrary.Delay` 0.5)
  (`PlayerController.SetViewTargetWithBlend` (`GameplayStatics.GetPlayerController` 0) (`GameplayStatics.GetPlayerPawn` 0) 1.0 "VTBlend_Linear" 0.0 false))

(event `self.TriggerBox.OnComponentBeginOverlap`
  (params (OverlappedComponent :type "PrimitiveComponent Object Reference") (OtherActor :type "Actor Object Reference") (OtherComp :type "PrimitiveComponent Object Reference") (OtherBodyIndex :type Integer) (bFromSweep :type Boolean) (SweepResult :type "HitResult Structure (by ref)"))
  (bind _angle (`/Game/MyActorMacroLibrary.AngleBetweenTwoVectors` (`self.GetActorForwardVector`) (`self.GetActorForwardVector` OtherActor))
    (:`Out`
      (if (< _angle 90.0)
        (message `/Game/Level4/BI_InformTeleport.InformTeleport` (`self.MyManager`) OtherActor self (`/Game/Level4/BP_PortalManager.PortalEnd` (`self.MyManager`)))
        (set `PrimitiveComponent.bGenerateOverlapEvents` false (`self.TriggerBox`))
        (`PrimitiveComponent.SetMaterial` (`self.Portal`) 0 "/Game/Level1/M_Tran.M_Tran")
        (set `self.CanPortal` false)
        (bind _outactors (`GameplayStatics.GetAllActorsWithInterface` "/Game/Level1/BI_Reset.BI_Reset_C"))
        (for _array_element _outactors
          (message `/Game/Level1/BI_Reset.Reset` _array_element))))))

(fn `UserConstructionScript`)