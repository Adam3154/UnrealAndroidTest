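; Carryable box actor that the player can pick up and put down, extending pickup logic from its parent class.
; PickUp caches the player pawn and enables Tick, which holds the box in front of the pawn with matching rotation.
; PutDown stops Tick and lowers the box along its up vector.
; Respawn resets transform, velocity, physics and picked state, but its height-check caller and the physics toggles in PickUp and PutDown are disconnected.
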(event `self.ReceiveBeginPlay`
  (`parent.ReceiveBeginPlay`)
  (`self.SetActorTickEnabled` false))

(event `self.ReceiveTick`
  (params (DeltaSeconds :type "Float (single-precision)"))
  (bind _playerpawn (`self.PlayerPawn`))
  (`self.K2_SetActorLocationAndRotation` (+ (`self.K2_GetActorLocation` _playerpawn) (* (`self.GetActorForwardVector` _playerpawn) 100.0)) (`self.K2_GetActorRotation` _playerpawn)))

(fn `PickUp`
  (`parent.PickUp`)
  (set `self.PlayerPawn` (`GameplayStatics.GetPlayerPawn` 0))
  (`self.SetActorTickEnabled` true))

(fn `PutDown`
  (`parent.PutDown`)
  (`self.SetActorTickEnabled` false)
  (`self.K2_SetActorLocation` (+ (`self.K2_GetActorLocation`) (* (`KismetMathLibrary.GetUpVector` (`self.K2_GetActorRotation`)) -50.0))))

(fn `Respawn`
  (params (Transform :type "Transform Structure"))
  (`self.K2_SetActorTransform` Transform)
  (`PrimitiveComponent.SetPhysicsLinearVelocity` (`self.StaticMesh`) (0.0 0.0 0.0) false "None")
  (`PrimitiveComponent.SetSimulatePhysics` (`self.StaticMesh`) false)
  (set `self.IsPicked` false))

(fn `UserConstructionScript`
  (`parent.UserConstructionScript`))