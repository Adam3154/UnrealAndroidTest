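; Exit-end portal actor in Level4 that teleports overlapping actors to the begin portal through BP_PortalManager.
; Once CanPortal is set, actors entering TriggerBox while facing into the portal are passed to the manager, then overlap events pause briefly to prevent retriggering.
; InformTrigger activates the portal in a short camera cutaway, swapping its material and enabling teleporting before blending the view back to the player.
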(event `self.ReceiveBeginPlay`
  (bind _outactors (`GameplayStatics.GetAllActorsOfClass` "/Game/Level4/BP_PortalManager.BP_PortalManager_C"))
  (set `self.MyManager` (`|GetArrayItem` _outactors)))

(event `self.TriggerBox.OnComponentBeginOverlap`
  (params (OverlappedComponent :type "PrimitiveComponent Object Reference") (OtherActor :type "Actor Object Reference") (OtherComp :type "PrimitiveComponent Object Reference") (OtherBodyIndex :type Integer) (bFromSweep :type Boolean) (SweepResult :type "HitResult Structure (by ref)"))
  (if (`self.CanPortal`)
    (bind _angle (`/Game/MyActorMacroLibrary.AngleBetweenTwoVectors` (`self.GetActorForwardVector` OtherActor) (`KismetMathLibrary.NegateVector` (`self.GetActorForwardVector`)))
      (:`Out`
        (if (< _angle 90.0)
          (message `/Game/Level4/BI_InformTeleport.InformTeleport` (`self.MyManager`) OtherActor self (`/Game/Level4/BP_PortalManager.PortalBegin` (`self.MyManager`)))
          (set `PrimitiveComponent.bGenerateOverlapEvents` false (`self.TriggerBox`))
          (`KismetSystemLibrary.Delay` 1.0)
          (set `PrimitiveComponent.bGenerateOverlapEvents` true (`self.TriggerBox`)))))))

(event `/Game/Level1/BI_InformTrigger.InformTrigger`
  (`PlayerController.SetViewTargetWithBlend` (`GameplayStatics.GetPlayerController` 0) (`self.Camera`) 1.0 "VTBlend_Linear" 0.0 false)
  (`KismetSystemLibrary.Delay` 1.5)
  (`PrimitiveComponent.SetMaterial` (`self.Portal`) 0 "/Game/Level4/M_PortalBegin.M_PortalBegin")
  (set `self.CanPortal` true)
  (`KismetSystemLibrary.Delay` 1.0)
  (`PlayerController.SetViewTargetWithBlend` (`GameplayStatics.GetPlayerController` 0) (`GameplayStatics.GetPlayerPawn` 0) 1.0 "VTBlend_Linear" 0.0 false))

(fn `UserConstructionScript`)