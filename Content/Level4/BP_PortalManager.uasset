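; Level 4 portal manager that drives the see-through view between PortalBegin and PortalEnd and handles teleporting between portals.
; BeginPlay caches the portals' relative rotation and disables Tick, as does Reset.
; When ticking, it mirrors the player camera's offset and rotation onto PortalEnd's SceneCapture; the reverse update is never called.
; InformTeleport moves an actor above the destination portal and turns player 0's control rotation by the portals' rotation difference.
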(event `/Game/Level1/BI_Reset.Reset`
  (`self.SetActorTickEnabled` false :!label _label))

(event `self.ReceiveBeginPlay`
  (set `self.RelativeRotation` (`KismetMathLibrary.NormalizedDeltaRotator` (`self.K2_GetActorRotation` (`self.PortalEnd`)) (`self.K2_GetActorRotation` (`self.PortalBegin`))))
  (goto _label))

(event `self.ReceiveTick`
  (params (DeltaSeconds :type "Float (single-precision)"))
  (`self.Portal BeginUpdate`))

(event `/Game/Level4/BI_InformTeleport.InformTeleport`
  (params (ActorToTele :type "Actor Object Reference") (Portal1 :type "Actor Object Reference") (Portal2 :type "Actor Object Reference"))
  (bind _returnvalue (`GameplayStatics.GetPlayerController` 0))
  ;[1 1 1] 传送
  (`self.K2_SetActorLocation` ActorToTele (+ (`self.K2_GetActorLocation` Portal2) (* (`KismetMathLibrary.GetUpVector` (`self.K2_GetActorRotation` Portal2)) (`self.HeightDiff`))) false false)
  ;;[1 1 1] 暂时没有重力转换时候的rotator
  (`Controller.SetControlRotation` _returnvalue (`KismetMathLibrary.ComposeRotators` (`Controller.GetControlRotation` _returnvalue) (`KismetMathLibrary.NormalizedDeltaRotator` (`self.K2_GetActorRotation` Portal2) (`self.K2_GetActorRotation` Portal1)))))

(fn `Portal BeginUpdate`
  (bind _portalend (`self.PortalEnd`))
  (bind _relativerotation (`self.RelativeRotation`))
  ;[1 1 1] 任意位置角度
  (`SceneComponent.K2_SetWorldLocationAndRotation` (`/Game/Level4/BP_PortalEnd.SceneCapture` _portalend) (+ (`self.K2_GetActorLocation` _portalend) (`KismetMathLibrary.GreaterGreater_VectorRotator` (- (`PlayerCameraManager.GetCameraLocation` (`GameplayStatics.GetPlayerCameraManager` 0)) (`self.K2_GetActorLocation` (`self.PortalBegin`))) _relativerotation)) (`KismetMathLibrary.ComposeRotators` (`PlayerCameraManager.GetCameraRotation` (`GameplayStatics.GetPlayerCameraManager` 0)) _relativerotation) false false))

(fn `PortalEndUpdate`
  (bind _portalbegin (`self.PortalBegin`))
  (bind _returnvalue (`KismetMathLibrary.NegateRotator` (`self.RelativeRotation`)))
  ;[1 1 1] 任意位置角度
  (`SceneComponent.K2_SetWorldLocationAndRotation` (`/Game/Level4/BP_PortalBegin.SceneCaptureComponent2D` _portalbegin) (+ (`self.K2_GetActorLocation` _portalbegin) (`KismetMathLibrary.GreaterGreater_VectorRotator` (- (`PlayerCameraManager.GetCameraLocation` (`GameplayStatics.GetPlayerCameraManager` 0)) (`self.K2_GetActorLocation` (`self.PortalEnd`))) _returnvalue)) (`KismetMathLibrary.ComposeRotators` (`PlayerCameraManager.GetCameraRotation` (`GameplayStatics.GetPlayerCameraManager` 0)) _returnvalue) false false))

(fn `UserConstructionScript`)