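; BP_TimeShadow is a ghost actor that replays a recorded movement track, then removes itself.
; On BeginPlay it caches the length of the MyStatus array, then steps through one entry per Tick.
; Each entry sets the actor's transform without sweep and writes the recorded speed into the movement component's velocity.
; When the entries run out, it destroys itself after a short delay.
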(event `self.ReceiveBeginPlay`
  (set `self.Length` (`KismetArrayLibrary.Array_Length` (`self.MyStatus`))))

(event `self.ReceiveTick`
  (params (DeltaSeconds :type "Float (single-precision)"))
  (bind (_transform _speed) (break `/Game/Level1/S_ActorStatus` (`|GetArrayItem` (`self.MyStatus`) (`self.Index`))))
  (if (< (`self.Index`) (`self.Length`))
    (`self.K2_SetActorTransform` (`|GetArrayItem` _transform))
    (set `MovementComponent.Velocity` (`|GetArrayItem` _speed) (`self.GetMovementComponent`))
    (`/Engine/EditorBlueprintResources/StandardMacros.IncrementInt` (`self.Index`))
    (else
      (`KismetSystemLibrary.Delay` 2.0)
      (`self.K2_DestroyActor`))))

(fn `UserConstructionScript`
  (`parent.UserConstructionScript`))